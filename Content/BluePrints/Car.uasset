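; Player car Blueprint that possesses itself on BeginPlay and simulates driving by moving a World actor instead of itself.
; Input actions set held flags, which Tick reads to shift World along its forward vector or yaw it by fixed per-frame steps, unscaled by delta time.
; Overlapping a DeadZone or exceeding MaxTimer opens Levelx1.
; Left/right push flags are set but unused, and PushLeft is never called.
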(event `self.ReceiveBeginPlay`
  ;[1 1 1] Setup as the Player
  (`Controller.Possess` (`GameplayStatics.GetPlayerController` 0) self))

(event `InputAction|PushForward`
  (params (Key :type "Key Structure"))
  (:`Pressed`
    (set `self.PushWorldForward` true))
  (:`Released`
    (set `self.PushWorldForward` false)))

(event `InputAction|PushLeft`
  (params (Key :type "Key Structure"))
  (:`Pressed`
    (set `self.PushWorldLeft` true))
  (:`Released`
    (set `self.PushWorldLeft` false)))

(event `InputAction|PushBackward`
  (params (Key :type "Key Structure"))
  (:`Pressed`
    (set `self.PushWorldBack` true))
  (:`Released`
    (set `self.PushWorldBack` false)))

(event `InputAction|PushRight`
  (params (Key :type "Key Structure"))
  (:`Pressed`
    (set `self.PushWorldRight` true))
  (:`Released`
    (set `self.PushWorldRight` false)))

(event `InputAction|RotateLeft`
  (params (Key :type "Key Structure"))
  (:`Pressed`
    (set `self.RotateWorldLeft` true))
  (:`Released`
    (set `self.RotateWorldLeft` false)))

(event `InputAction|RotateRight`
  (params (Key :type "Key Structure"))
  (:`Pressed`
    (set `self.RotateWorldRight` true))
  (:`Released`
    (set `self.RotateWorldRight` false)))

(event `self.ReceiveActorBeginOverlap`
  (params (OtherActor :type "Actor Object Reference"))
  (cast `/Game/BluePrints/DeadZone` OtherActor)
  (if true
    (`GameplayStatics.OpenLevel` "Levelx1")))

(event `self.ReceiveTick`
  (params (DeltaSeconds :type "Float (single-precision)"))
  (`self.PushForward` -20.0 (`self.PushWorldForward`))
  (`self.PushForward` 20.0 (`self.PushWorldBack`))
  (`self.RotateLeft`)
  (`self.RotateRight`)
  ;[1 1 1] Outside Max Time
  (if (> (`GameplayStatics.GetTimeSeconds`) (`self.MaxTimer`))
    (`GameplayStatics.OpenLevel` "Levelx1")))

(fn `PushForward`
  (params (Amount :type "Float (double-precision)") (Condition :type Boolean))
  (bind _world (`self.World`))
  (if Condition
    (`self.K2_SetActorLocation` _world (+ (`self.K2_GetActorLocation` _world) (* (`self.GetActorForwardVector` _world) Amount)) false false)))

(fn `PushLeft`
  (params (Direction :type "Float (double-precision)") (Condition :type Boolean))
  (bind _world (`self.World`))
  (if Condition
    (`self.K2_SetActorLocation` _world (+ (`self.K2_GetActorLocation` _world) (* (`self.GetActorRightVector` _world) Direction)) false false)))

(fn `RotateLeft`
  (bind _world (`self.World`))
  (bind (_returnvalue_roll _returnvalue_pitch _returnvalue_yaw) (`KismetMathLibrary.BreakRotator` (`self.K2_GetActorRotation` _world)))
  (if (`self.RotateWorldLeft`)
    (`self.K2_SetActorRotation` _world (`KismetMathLibrary.MakeRotator` _returnvalue_roll _returnvalue_pitch (+ _returnvalue_yaw 0.4)) false)))

(fn `RotateRight`
  (bind _world (`self.World`))
  (bind (_returnvalue_roll _returnvalue_pitch _returnvalue_yaw) (`KismetMathLibrary.BreakRotator` (`self.K2_GetActorRotation` _world)))
  (if (`self.RotateWorldRight`)
    (`self.K2_SetActorRotation` _world (`KismetMathLibrary.MakeRotator` _returnvalue_roll _returnvalue_pitch (+ _returnvalue_yaw -0.4)) false)))

(fn `UserConstructionScript`)